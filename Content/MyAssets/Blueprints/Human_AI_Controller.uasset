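; AI controller for HumanBP that patrols waypoints and watches for the player.
; It loops through the pawn's places with AIMoveTo and short pauses.
; Two perception components (front and 360º) plus a delayed Tick recheck feed CheckIfSeePlayer, which stops movement and flags WatchingPlayer when a detectable Player-tagged actor is sensed, otherwise resuming patrol.
; When the human dies, detection checks cease and the watching and movement flags clear.
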(event OnTargetPerceptionUpdated(AIPerception)
  (params (Actor :type Actor%20Object%20Reference) (Stimulus :type AI%20Stimulus%20Structure))
  ;[1 1 1] Check If See Player
  ;;[1 1 1] Check In Front
  (bind _ashuman_bp (Utilities|Casting|CastToHumanBP (Pawn|GetControlledPawn)))
  (bind _alive_ (Default|GetAlive _ashuman_bp))
  (if _alive_
    (CallFunction|CheckifSeePlayer Actor (.bsuccessfullysensed Stimulus))))

(event OnTargetPerceptionUpdated(AIPerception1)
  (params (Actor :type Actor%20Object%20Reference) (Stimulus :type AI%20Stimulus%20Structure))
  ;[1 1 1] Check If See Player
  ;;[1 1 1] Check In 360º
  (bind _ashuman_bp (Utilities|Casting|CastToHumanBP (Pawn|GetControlledPawn)))
  (bind _alive_ (Default|GetAlive _ashuman_bp))
  (if _alive_
    (CallFunction|CheckifSeePlayer Actor (.bsuccessfullysensed Stimulus))))

(event Custom|GoNextStep
  ;[1 1 1] MovmentControll
  (AI|AIMoveTo 0 (Utilities|Array|Get(acopy) (Variables|Default|GetPlacesToGo) (Variables|Default|GetPlaceToGoIndex)) 0 1.0 false
    (:OnSuccess
      (Utilities|FlowControl|Delay 2.0)
      (CallFunction|NextPlacetoGo)
      (CallFunction|GoNextStep))))

(event EventBeginPlay
  ;[1 1 1] Start
  (bind _ashuman_bp (Utilities|Casting|CastToHumanBP (Pawn|GetControlledPawn)))
  (bind _placestogo (Default|SetPlaces _ashuman_bp))
  (Variables|Default|SetPlacesToGo _placestogo)
  (CallFunction|GoNextStep)
  (Variables|Default|SetCurrentTimeToCheck (Variables|Default|GetTimeToCheckIfSomeoneThere)))

(event EventTick
  (params (DeltaSeconds :type Float%20%28single-precision%29))
  (bind _returnvalue (Pawn|GetControlledPawn))
  (bind _actor (Variables|Default|GetActor))
  ;[1 1 1] Check If See Player
  (bind _ashuman_bp (Utilities|Casting|CastToHumanBP (Pawn|GetControlledPawn)))
  (bind _alive_ (Default|GetAlive _ashuman_bp))
  (if _alive_
    (Utilities|FlowControl|Delay (Variables|Default|GetCurrentTimeToCheck))
    (Utilities|IsValid _actor
      (:Is%20Valid
        (CallFunction|CheckifSeePlayer _actor (or (.bsuccessfullysensed (stale OnTargetPerceptionUpdated(AIPerception1) Stimulus)) (.bsuccessfullysensed (stale OnTargetPerceptionUpdated(AIPerception) Stimulus))))))
    (else
      ;;[1 1 1] Stop Everything when die
      (Variables|Default|SetCanMove false)
      (Development|PrintString (Utilities|GetDisplayName _returnvalue) true true "(R=1.000000,G=0.009094,B=0.000000,A=1.000000)" 3e+01)
      (Development|PrintString "ESTA MUERTO" true true "(R=1.000000,G=0.000000,B=0.007639,A=1.000000)" 3e+01)
      (bind _ashuman_bp_2 (Utilities|Casting|CastToHumanBP _returnvalue))
      (Default|SetWatchingPlayer _ashuman_bp_2 false)
      (Variables|Default|SetAI_Alive false))))

(fn ConstructionScript)

(fn NextPlacetoGo
  (Math|Integer|IncrementInt (Variables|Default|GetPlaceToGoIndex)
    (:%20%20
      (if (>= (Variables|Default|GetPlaceToGoIndex) (Utilities|Array|Length (Variables|Default|GetPlacesToGo)))
        (Variables|Default|SetPlaceToGoIndex 0)))))

(fn CheckifSeePlayer
  (params (Actor :type Actor%20Object%20Reference) (StimulsSuccesfullSensed :type Boolean))
  (bind _returnvalue (Pawn|GetControlledPawn))
  (if (and StimulsSuccesfullSensed (Actor|ActorHasTag Actor "Player"))
    ;[1 1 1] Check If Player Can Be Watched
    (bind _output_get (Variables|Default|SetActor Actor))
    (bind _asfirst_person_character (Utilities|Casting|CastToFirstPersonCharacter _output_get))
    (bind _isseen (Default|GettingWatched _asfirst_person_character))
    (if _isseen
      ;[1 1 1] Watching Player
      (bind _ashuman_bp (Utilities|Casting|CastToHumanBP _returnvalue))
      (Default|SetWatchingPlayer _ashuman_bp true)
      (AI|Navigation|StopMovement)
      (Variables|Default|SetCanMove false)
      (Variables|Default|SetCurrentTimeToCheck (Variables|Default|GetTimeToCheckIfPlayerThere))
      (else
        ;[1 1 1] Watching player But Invisible or Save
        (bind _ashuman_bp_2 (Utilities|Casting|CastToHumanBP _returnvalue))
        (Default|SetWatchingPlayer _ashuman_bp_2 false)
        (CallFunction|CheckifIsStoppedMove)))
    (else
      ;[1 1 1] Not Watching Player
      (bind _ashuman_bp_3 (Utilities|Casting|CastToHumanBP (Pawn|GetControlledPawn)))
      (Default|SetWatchingPlayer _ashuman_bp_3 false)
      (CallFunction|CheckifIsStoppedMove))))

(fn CheckifIsStoppedMove
  (if (not (Variables|Default|GetCanMove))
    (Variables|Default|SetCanMove true)
    (Variables|Default|SetCurrentTimeToCheck (Variables|Default|GetTimeToCheckIfSomeoneThere))
    (CallFunction|GoNextStep)))