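; Human NPC that can be burned to death and reports to the player character when it is watching them.
; Tick updates a player-facing health bar, drains HP while burning and toggles custom depth when the player's focus check passes.
; Externally set watching state is forwarded to FirstPersonCharacter, and a living human turns toward the player.
; Death removes the health bar, applies a burned material, disables capsule collision and clears the AI controller class.
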(event EventTick
  (params (DeltaSeconds :type Float%20%28single-precision%29))
  (CallFunction|SetHealthBar)
  (CallFunction|GettingBurned)
  (CallFunction|CheckifDead)
  (CallFunction|CheckifPlayerFocused)
  (CallFunction|DamagePlayerifSeen))

(fn ConstructionScript)

(fn SetPlaces
  (return (Variables|Default|GetPointToGo)))

(fn SetBurn
  (params (Burn? :type Boolean))
  (Variables|Default|SetisBurning Burn?))

(fn GetAlive
  (return (Variables|Default|GetisAlive)))

(fn GetWatchingPlayer
  (return (Variables|Default|GetisWatchingPlayer)))

(fn SetWatchingPlayer
  (params (WatchingPlayer? :type Boolean))
  (Variables|Default|SetisWatchingPlayer WatchingPlayer?)
  (return))

(fn SetHealthBar
  (bind _widget (Variables|Default|GetWidget))
  (bind _widget_2 (Variables|Default|GetWidget))
  ;[1 1 1] Set HealthBar
  (Utilities|IsValid _widget
    (:Is%20Valid
      (bind _ashuman_widget (Utilities|Casting|CastToHumanWidget (UserInterface|GetUserWidgetObject _widget)))
      (Progress|SetPercent (Variables|/Game/MyAssets/Others/Widgets/HumanWidget.HumanWidget_C|GetHealthBar _ashuman_widget) (/ (Variables|Default|GetHP) 1e+02))
      (Transformation|SetWorldRotation _widget_2 (Math|Rotator|FindLookatRotation (Transformation|GetWorldLocation _widget_2) (Transformation|GetActorLocation (Game|GetPlayerCharacter 0))) false false))))

(fn GettingBurned
  ;[1 1 1] GettingBurned
  (if (Variables|Default|GetisBurning)
    (Variables|Default|SetHP (- (Variables|Default|GetHP) (/ (Variables|Default|GetBurnHPConsume) 1e+02)))))

(fn CheckifDead
  ;[1 1 1] Is Dead
  (if (and (<= (Variables|Default|GetHP) 0.0) (Variables|Default|GetisAlive))
    (Components|DestroyComponent (Variables|Default|GetWidget))
    (Variables|Default|SetisAlive false)
    (Rendering|Material|SetMaterial (Variables|Character|GetMesh) 0 "/Game/MyAssets/Materials/BurnedMaterial.BurnedMaterial")
    (Collision|SetCollisionEnabled (Variables|Collision|GetCapsuleComponent) "NoCollision")
    (Variables|Default|SetAIControllerClass 0)))

(fn CheckifPlayerFocused
  (bind _mesh (Variables|Character|GetMesh))
  ;[1 1 1] Player Focused
  (bind _asfirst_person_character (Utilities|Casting|CastToFirstPersonCharacter (Game|Player|GetPlayerPawn 0)))
  (bind _isfocused_ (Default|CheckifFocus _asfirst_person_character))
  (if (and _isfocused_ (Variables|Default|GetisAlive))
    (Rendering|SetRenderCustomDepth _mesh true)
    (else
      (Rendering|SetRenderCustomDepth _mesh false))))

(fn DamagePlayerifSeen
  (bind _returnvalue (Game|Player|GetPlayerPawn 0))
  (if (Variables|Default|GetisWatchingPlayer)
    ;[1 1 1] Set Player Is Getting Watched
    (bind _asfirst_person_character (Utilities|Casting|CastToFirstPersonCharacter _returnvalue))
    (Default|SetifWatchingPlayer _asfirst_person_character true)
    (Variables|Default|SetSeenBefore true)
    (if (Variables|Default|GetisAlive)
      ;[1 1 1] Look At Player When Scared
      (Transformation|SetWorldRotation (Variables|Transformation|GetRootComponent) (Math|Rotator|FindLookatRotation (Transformation|GetActorLocation) (Transformation|GetActorLocation (Game|Player|GetPlayerPawn 0))) false false))
    (else
      ;[1 1 1] Set Player Is Not Getting Watched
      (if (Variables|Default|GetSeenBefore)
        (bind _asfirst_person_character_2 (Utilities|Casting|CastToFirstPersonCharacter _returnvalue))
        (Default|SetifWatchingPlayer _asfirst_person_character_2 false)
        (Variables|Default|SetSeenBefore false)))))