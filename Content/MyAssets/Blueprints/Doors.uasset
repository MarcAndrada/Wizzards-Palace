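; Doors Blueprint with a trigger box that marks when the player is inside its volume by toggling the character's Save flag.
; Begin and end overlap check the other component for the Player tag, print a debug message, then cast the actor to FirstPersonCharacter.
; The cast result receives Save as true on entry and false on exit; the graphs contain no door movement logic.
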(event OnComponentBeginOverlap(Box)
  (params (OverlappedComponent :type Primitive%20Component%20Object%20Reference) (OtherActor :type Actor%20Object%20Reference) (OtherComp :type Primitive%20Component%20Object%20Reference) (OtherBodyIndex :type Integer) (bFromSweep :type Boolean) (SweepResult :type Hit%20Result%20Structure%20%28by%20ref%29))
  (if (Components|ComponentHasTag OtherComp "Player")
    (Development|PrintString "You son of a bitch im in")
    (bind _asfirst_person_character (Utilities|Casting|CastToFirstPersonCharacter OtherActor))
    (Default|SetSave _asfirst_person_character true)))

(event OnComponentEndOverlap(Box)
  (params (OverlappedComponent :type Primitive%20Component%20Object%20Reference) (OtherActor :type Actor%20Object%20Reference) (OtherComp :type Primitive%20Component%20Object%20Reference) (OtherBodyIndex :type Integer))
  (if (Components|ComponentHasTag OtherComp "Player")
    (Development|PrintString "You son of a bitch im out")
    (bind _asfirst_person_character (Utilities|Casting|CastToFirstPersonCharacter OtherActor))
    (Default|SetSave _asfirst_person_character false)))

(fn ConstructionScript)