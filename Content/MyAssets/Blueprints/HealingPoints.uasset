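; HealingPoints is a healing zone that tells the first-person character when it enters or leaves the area.
; Box overlap begin and end events accept components tagged Player but not Fire, then cast the actor to FirstPersonCharacter.
; Each event calls SetHealingZone with the in-zone state, Smoke particles and Box, leaving any healing logic to the character.
; Debug strings in Spanish print on entry and exit.
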(event OnComponentBeginOverlap(Box)
  (params (OverlappedComponent :type Primitive%20Component%20Object%20Reference) (OtherActor :type Actor%20Object%20Reference) (OtherComp :type Primitive%20Component%20Object%20Reference) (OtherBodyIndex :type Integer) (bFromSweep :type Boolean) (SweepResult :type Hit%20Result%20Structure%20%28by%20ref%29))
  (if (and (Components|ComponentHasTag OtherComp "Player") (not (Components|ComponentHasTag OtherComp "Fire")))
    (bind _asfirst_person_character (Utilities|Casting|CastToFirstPersonCharacter OtherActor))
    (Default|SetHealingZone _asfirst_person_character true (Variables|Default|GetSmoke) (Variables|Default|GetBox))
    (Development|PrintString "Esta dentro")))

(event OnComponentEndOverlap(Box)
  (params (OverlappedComponent :type Primitive%20Component%20Object%20Reference) (OtherActor :type Actor%20Object%20Reference) (OtherComp :type Primitive%20Component%20Object%20Reference) (OtherBodyIndex :type Integer))
  (if (and (Components|ComponentHasTag OtherComp "Player") (not (Components|ComponentHasTag OtherComp "Fire")))
    (bind _asfirst_person_character (Utilities|Casting|CastToFirstPersonCharacter OtherActor))
    (Default|SetHealingZone _asfirst_person_character false (Variables|Default|GetSmoke) (Variables|Default|GetBox))
    (Development|PrintString "Adios")))

(fn ConstructionScript)